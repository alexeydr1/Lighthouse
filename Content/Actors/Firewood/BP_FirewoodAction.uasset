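; Interactive firewood-chopping station, a timed-swing minigame that starts when the player overlaps its sphere.
; Overlap locks movement, turns the camera to the target and creates a progress-bar widget, with a stepped world-space tutorial gating the first attempt.
; Action presses start and stop the bar, which rotates the axe as it changes.
; The stopped value decides the timeline-driven swing's outcome: success spawns small firewood, while either result plays its own effect and sound.
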(event OnComponentBeginOverlap(Sphere)
  (params (OverlappedComponent :type Primitive%20Component%20Object%20Reference) (OtherActor :type Actor%20Object%20Reference) (OtherComp :type Primitive%20Component%20Object%20Reference) (OtherBodyIndex :type Integer) (bFromSweep :type Boolean) (SweepResult :type Hit%20Result%20Structure%20%28by%20ref%29))
  (bind _returnvalue (Game|GetPlayerCharacter 0))
  (if (== OtherActor _returnvalue)
    (bind _returnvalue_2 (UserInterface|CreateWidget "/Game/UMG/WBP_ProgressBar.WBP_ProgressBar_C" 0 self))
    (bind _output_get (Variables|Default|SetProgressBarWidget _returnvalue_2))
    (UserInterface|Viewport|AddtoViewport _output_get 0)
    (CallFunction|StartActionInteraction)
    (Components|Activation|Deactivate (Variables|/Script/Engine.Character|GetCharacterMovement _returnvalue))
    (bind _asbp_third_person_character (Utilities|Casting|CastToBP_ThirdPersonCharacter _returnvalue))
    (Default|RotateCameratoTarget _asbp_third_person_character (Transformation|GetWorldLocation (Variables|Default|GetTarget)) self)))

(event Custom|TryHit
  (bind _progressbarwidget (Variables|Default|GetProgressBarWidget))
  (Utilities|IsValid _progressbarwidget
    (:Is%20Valid
      (if (Variables|/Game/UMG/WBP_ProgressBar.WBP_ProgressBar_C|GetbIsProgressStarted _progressbarwidget)
        (bind _resultvalue (Default|StopProgress _progressbarwidget))
        (CallFunction|PlayHitAnimation _resultvalue)
        (else
          (Default|StartProgress _progressbarwidget))))))

(event Custom|PlayHitAnimation
  (params (Value :type Float%20%28double-precision%29))
  (bind _firewoodsystem (Variables|Default|GetFirewoodSystem))
  (bind _axe (Variables|Default|GetAxe))
  (Variables|Default|SetSoundIsPlayed false)
  (Variables|Default|SetIsSuccessfullhit (<= (Variables|Default|GetPrecentForSuccess) Value))
  (Variables|Default|SetIsHitAnimationStarted true)
  (Variables|Default|SetRotatorBeforeHit (Variables|/Script/Engine.SceneComponent|GetRelativeRotation _axe))
  (Variables|Default|SetLocationBeforeHit (Variables|/Script/Engine.SceneComponent|GetRelativeLocation _axe))
  (Audio|PlaySoundatLocation "/Game/Sounds/Firewoods/AxeHitPrepare.AxeHitPrepare" "0, 0, 0" "0, 0, 0" 1.0 1.0 0.0 0 0 0 0)
  (bind _newtrack_0 (Timeline|Timeline PlayFromStart)
    (:Update
      (Transformation|SetRelativeLocationAndRotation (Variables|Default|GetAxe) (Math|Vector|Lerp(Vector) (Variables|Default|GetAxeStartActionLocation) (Variables|Default|GetAxeLocationOnEndHitAnimation) _newtrack_0) (Math|Rotator|Lerp(Rotator) (Variables|Default|GetRotatorBeforeHit) (Math|Rotator|SelectRotator (Variables|Default|GetAxeRotationOnEndHitAnimation) "-12.000000,0.000000,0.000000" (Variables|Default|GetIsSuccessfullhit)) _newtrack_0 true) false false)
      (if (and (>= _newtrack_0 0.9) (not (Variables|Default|GetSoundIsPlayed)))
        (Variables|Default|SetSoundIsPlayed true)
        (if (Variables|Default|GetIsSuccessfullhit)
          (Audio|PlaySound2D "/Game/Sounds/Firewoods/Success.Success" 1.0 1.0 0.0 0 0)
          (Class|NiagaraComponent|SetAsset _firewoodsystem "/Game/Niagara/Firewood/FirewoodSystem.FirewoodSystem" true)
          (Components|Activation|Activate _firewoodsystem true)
          (Rendering|SetVisibility (Variables|Default|GetTarget) false false)
          (Game|SpawnActorfromClass "/Game/Actors/Firewood/BP_SmallFirewood.BP_SmallFirewood_C" (Math|Transform|MakeTransform (+ (Transformation|GetWorldLocation (Variables|Default|GetDefaultSceneRoot)) "148.000000,10.000000,-2.000000")) "Undefined" "MultiplyWithRoot" 0 0)
          (else
            (Audio|PlaySound2D "/Game/Sounds/Firewoods/Unsuccessfull.Unsuccessfull" 1.0 1.0 0.0 0 0)
            (Class|NiagaraComponent|SetAsset _firewoodsystem "/Game/Niagara/Firewood/FirewoodSystemSmall.FirewoodSystemSmall" true)
            (Components|Activation|Activate _firewoodsystem true)))
        (Variables|Default|SetIsHitAnimationStarted false)))))

(event EventOnCameraRotationCompleted
  (Transformation|SetRelativeLocationAndRotation (Variables|Default|GetAxe) (Variables|Default|GetAxeStartActionLocation) "0, 0, 0" false false)
  (if (not (Variables|Default|GetTutorialCompleted))
    (Rendering|SetVisibility (Variables|Default|GetWidgetTutorial) true false)))

(event EventTick
  (params (DeltaSeconds :type Float%20%28single-precision%29))
  (bind _widgettutorial (Variables|Default|GetWidgetTutorial))
  (if (Rendering|IsVisible _widgettutorial)
    (Transformation|SetRelativeRotation (Variables|Default|GetWidgetTutorial) (Math|Rotator|CombineRotators (Math|Rotator|FindLookatRotation (Transformation|GetSocketLocation (Variables|/Script/Engine.Character|GetMesh (Game|GetPlayerCharacter 0)) "head") (Transformation|GetWorldLocation _widgettutorial)) "0.000000,180.000000,0.000000") false false)))

(event EventBeginPlay
  (bind _aswbp_tutorial (Utilities|Casting|CastToWBP_Tutorial (UserInterface|GetUserWidgetObject (Variables|Default|GetWidgetTutorial))))
  (Default|SetStadies _aswbp_tutorial (Variables|Default|GetTutorialStadies)))

(fn ConstructionScript)

(fn OnCancelPressed
  (CallFunction|StopActionInteraction)
  (Components|Activation|Activate (Variables|/Script/Engine.Character|GetCharacterMovement (Game|GetPlayerCharacter 0)) false)
  (Rendering|SetVisibility (Variables|Default|GetTarget) false false)
  (Transformation|SetRelativeLocationAndRotation (Variables|Default|GetAxe) (Variables|Default|GetAxeBaseLocation) "0, 0, 0" false false)
  (bind _progressbarwidget (Variables|Default|GetProgressBarWidget)
    (:then
      (Widget|RemovefromParent _progressbarwidget))
    (:else)))

(fn OnActionPressed
  (if (not (Variables|Default|GetIsHitAnimationStarted))
    (if (Variables|Default|GetTutorialCompleted)
      (Rendering|SetVisibility (Variables|Default|GetTarget) true false)
      (CallFunction|TryHit)
      (else
        (bind _aswbp_tutorial (Utilities|Casting|CastToWBP_Tutorial (UserInterface|GetUserWidgetObject (Variables|Default|GetWidgetTutorial))))
        (bind _output_get (Variables|Default|SetTutorialCompleted (Default|ShowNextStadies _aswbp_tutorial)))
        (if _output_get
          (Rendering|SetVisibility (Variables|Default|GetWidgetTutorial) false false))))))

(fn OnPercentProgressBarWidgetChanged
  (params (NewValue :type Float%20%28double-precision%29))
  (Transformation|SetRelativeRotation (Variables|Default|GetAxe) (Math|Rotator|Lerp(Rotator) "0, 0, 0" "90.000000,0.000000,0.000000" NewValue true) false false))