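; Base actor for player-driven action interactions, meant to be extended through empty hook functions.
; StartActionInteraction and StopActionInteraction set the ActionStarted flag and add or remove the IMC_ActionMapping Enhanced Input context on player 0.
; While the flag is set, the IA_Action and IA_Cancel Started events call OnActionPressed and OnCancelPressed.
; OnPercentProgressBarWidgetChanged is another empty hook, taking a new value.
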(event Input|EnhancedActionEvents|EnhancedInputActionIA_Cancel
  (params (ActionValue :type Boolean) (ElapsedSeconds :type Float%20%28double-precision%29) (TriggeredSeconds :type Float%20%28double-precision%29) (InputAction :type Input%20Action%20Object%20Reference :default "/Game/IMC/IA_Cancel.IA_Cancel"))
  (:Started
    (if (Variables|Default|GetActionStarted)
      (CallFunction|OnCancelPressed))))

(event Input|EnhancedActionEvents|EnhancedInputActionIA_Action
  (params (ActionValue :type Boolean) (ElapsedSeconds :type Float%20%28double-precision%29) (TriggeredSeconds :type Float%20%28double-precision%29) (InputAction :type Input%20Action%20Object%20Reference :default "/Game/IMC/IA_Action.IA_Action"))
  (:Started
    (if (Variables|Default|GetActionStarted)
      (CallFunction|OnActionPressed))))

(fn ConstructionScript)

(fn StartActionInteraction
  (Variables|Default|SetActionStarted true)
  (Input|AddMappingContext (PlayerController|LocalPlayerSubsystems|GetEnhancedInputLocalPlayerSubsystem (Game|GetPlayerController 0)) "/Game/IMC/IMC_ActionMapping.IMC_ActionMapping" 0 "(bIgnoreAllPressedKeysUntilRelease=True,bForceImmediately=False,bNotifyUserSettings=False)"))

(fn StopActionInteraction
  (Variables|Default|SetActionStarted false)
  (Input|RemoveMappingContext (PlayerController|LocalPlayerSubsystems|GetEnhancedInputLocalPlayerSubsystem (Game|GetPlayerController 0)) "/Game/IMC/IMC_ActionMapping.IMC_ActionMapping" "(bIgnoreAllPressedKeysUntilRelease=True,bForceImmediately=False,bNotifyUserSettings=False)"))

(fn OnActionPressed)

(fn OnCancelPressed)

(fn OnPercentProgressBarWidgetChanged
  (params (NewValue :type Float%20%28double-precision%29)))