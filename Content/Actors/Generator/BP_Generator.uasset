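; Interactable generator actor that the player switches on and off, with a spinning rotor, smoke and start-then-running audio.
; A looping timer randomly breaks it while it runs, and BrokeIndex then selects rotor speed, smoke, sound and whether it can restart.
; The random range currently always picks fault 3, which shuts it down, blocks restarting and shows Niagara sparks at a random point with electrical audio.
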(event OnComponentBeginOverlap(Sphere)
  (params (OverlappedComponent :type Primitive%20Component%20Object%20Reference) (OtherActor :type Actor%20Object%20Reference) (OtherComp :type Primitive%20Component%20Object%20Reference) (OtherBodyIndex :type Integer) (bFromSweep :type Boolean) (SweepResult :type Hit%20Result%20Structure%20%28by%20ref%29))
  (if (== OtherActor (Game|GetPlayerCharacter 0))
    (CallFunction|StartActionInteraction)))

(event Custom|OnElectricCompleted
  (bind _electricaudio (Variables|Default|GetElectricAudio))
  (Audio|Components|Audio|Play _electricaudio (Math|Random|RandomFloatinRange 0.0 (Variables|/Script/Engine.SoundBase|GetDuration (Variables|/Script/Engine.AudioComponent|GetSound _electricaudio)))))

(event Custom|SelectBreake
  (bind _audio (Variables|Default|GetAudio))
  (Audio|Components|Audio|SetSound _audio "/Game/Sounds/Generator/Broke.Broke")
  (Audio|Components|Audio|Play _audio 0.0)
  (CallFunction|StartRandomBroke))

(event Custom|StartGenerator
  (bind _sound (CallFunction|GetSoundbyBroke))
  (bind _sound_2 (CallFunction|GetSoundbyBroke))
  (bind _audio (Variables|Default|GetAudio))
  (if (not (Variables|Default|GetbIsWorked))
    (Effects|Components|ParticleSystem|SetTemplate (Variables|Default|GetP_Smoke_A) (CallFunction|GetParticlebyBroke))
    (if (or (not (Variables|Default|GetbIsBroken)) (CallFunction|GetCanStartbyBroke))
      (Variables|Default|SetbIsWorked true)
      (Audio|Components|Audio|SetSound _audio (select (Utilities|IsValid _sound_2) _sound_2 "/Game/Sounds/Generator/StartGenerator.StartGenerator"))
      (Audio|Components|Audio|Play _audio 0.0)
      (Utilities|FlowControl|Sequence
        (:then_1
          (Utilities|FlowControl|RetriggerableDelay 1.68)
          (if (Variables|Default|GetbIsWorked)
            (Audio|Components|Audio|SetSound _audio (select (Utilities|IsValid _sound) _sound "/Game/Sounds/Generator/WorkedGenerator.WorkedGenerator"))
            (Audio|Components|Audio|Play _audio 0.0)))))))

(event Custom|IsNeedBreakeGenerator
  (if (and (Variables|Default|GetbIsWorked) (not (Variables|Default|GetbIsBroken)))
    (if (<= (Math|Random|RandomFloatinRange 0.0 1e+02) (Variables|Default|GetBreakingChance))
      (CallFunction|SelectBreake))))

(event Custom|DisableGenerator
  (Variables|Default|SetbIsWorked false)
  (Audio|Components|Audio|SetSound (Variables|Default|GetAudio) 0)
  (Effects|Particles|Trails|EndTrails (Variables|Default|GetP_Smoke_A)))

(event EventBeginPlay
  (Utilities|Time|SetTimerbyEvent (delegate Custom|IsNeedBreakeGenerator) 5.0 true))

(event EventTick
  (params (DeltaSeconds :type Float%20%28single-precision%29))
  (bind _rotor (Variables|Default|GetRotor))
  (if (Variables|Default|GetbIsWorked)
    (if (Variables|Default|GetbIsBroken)
      (Transformation|AddWorldRotation _rotor (Math|Rotator|MakeRotator 0.0 (CallFunction|GetRotateSpeedbyBroke) 0.0) false false)
      (else
        (Transformation|AddWorldRotation _rotor "10.000000,0.000000,0.000000" false false)))))

(fn ConstructionScript)

(fn StartRandomBroke
  (bind _electricaudio (Variables|Default|GetElectricAudio))
  (Variables|Default|SetBrokeIndex (Math|Random|RandomIntegerinRange 3 3))
  (Variables|Default|SetbIsBroken true)
  (switch int (Variables|Default|GetBrokeIndex)
    (:0
      (Effects|Components|ParticleSystem|SetTemplate (Variables|Default|GetP_Smoke_A) "/Game/Realistic_Starter_VFX_Pack_Vol2/Particles/Smoke/P_Smoke_B.P_Smoke_B"))
    (:1
      (CallFunction|DisableGenerator))
    (:3
      (CallFunction|DisableGenerator)
      (Rendering|SetVisibility (Variables|Default|GetNiagara) true true)
      (Components|Activation|SetActive _electricaudio true true)
      (EventDispatchers|BindEventtoOnAudioFinished _electricaudio (EventDispatchers|CreateEvent :!event Custom|OnElectricCompleted))
      (Transformation|SetRelativeLocation (Variables|Default|GetNiagara) (.OutItem (Utilities|Array|Random (Variables|Default|GetElectricLocations))) false false))))

(fn OnActionPressed
  (|CallParentFunction)
  (if (Variables|Default|GetbIsWorked)
    (CallFunction|DisableGenerator)
    (Audio|PlaySound2D "/Game/Sounds/Generator/DisableGenerator.DisableGenerator" 1.0 1.0 0.0 0 0)
    (else
      (CallFunction|StartGenerator)
      (Audio|PlaySound2D "/Game/Sounds/Generator/EnableGenerator.EnableGenerator" 1.0 1.0 0.0 0 0))))

(fn OnCancelPressed
  (|CallParentFunction))

(fn GetParticlebyBroke
  (return (Utilities|Select :Index (Variables|Default|GetBrokeIndex) :Option%200 "/Game/Realistic_Starter_VFX_Pack_Vol2/Particles/Smoke/P_Smoke_B.P_Smoke_B" :Option%201 "/Game/Realistic_Starter_VFX_Pack_Vol2/Particles/Smoke/P_Smoke_A.P_Smoke_A")))

(fn GetRotateSpeedbyBroke
  (return (Utilities|Select :Index (Variables|Default|GetBrokeIndex) :Option%200 1e+01 :Option%201 0.0 :Option%202 0.3 :Option%203 0.0)))

(fn GetCanStartbyBroke
  (return (Utilities|Select :Index (Variables|Default|GetBrokeIndex) :Option%200 true :Option%201 false :Option%202 true :Option%203 false)))

(fn GetSoundbyBroke
  (return (Utilities|Select :Index (Variables|Default|GetBrokeIndex) :Option%200 "/Game/Sounds/Generator/Broke.Broke" :Option%201 0 :Option%202 "/Game/Sounds/Generator/Broke.Broke" :Option%203 0)))